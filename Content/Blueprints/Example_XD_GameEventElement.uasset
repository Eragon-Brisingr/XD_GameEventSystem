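; An example game event element that serves as a "reach target" objective, completed when the event owner character overlaps the target actor.
; On activation it binds the character's actor overlap events and finishes immediately if the character is already inside the target, then unbinds them on deactivation.
; Beginning overlap with the target finishes the element, ending it calls SetReactive, and the description shows the target's name and completion state.
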(event Custom|WhenEndOverlap
  (params (OverlappedActor :type Actor%20Object%20Reference) (OtherActor :type Actor%20Object%20Reference))
  (if (Class|XDObjectFunctionLibrary|Equal(Object) OtherActor (Variables|Default|Get目标))
    (Class|XDGameEventElementBase|SetReactive)))

(event Custom|WhenBeginOverlap
  (params (OverlappedActor :type Actor%20Object%20Reference) (OtherActor :type Actor%20Object%20Reference))
  (if (Class|XDObjectFunctionLibrary|Equal(Object) OtherActor (Variables|Default|Get目标))
    (Class|XDGameEventElementBase|FinishGameEventElement)))

(event EventWhenActivateGameEventElement
  (params (GameEventOwnerCharacter :type Pawn%20Object%20Reference) (GameEventOwner :type Controller%20Object%20Reference))
  (EventDispatchers|AssignOnActorBeginOverlap GameEventOwnerCharacter (delegate Custom|WhenBeginOverlap))
  (EventDispatchers|AssignOnActorEndOverlap GameEventOwnerCharacter (delegate Custom|WhenEndOverlap))
  ;[1 1 1] 添加判断，假如该Actor激活游戏事件时就在体积内
  (if (Utilities|Array|ContainsItem (Collision|GetOverlappingActors (Utilities|ResolveSoftReference (Variables|Default|Get目标)) (Utilities|GetClass GameEventOwnerCharacter) :!class /Script/Engine.Actor) GameEventOwnerCharacter)
    (Class|XDGameEventElementBase|FinishGameEventElement)))

(event EventWhenUnactiveGameEventElement
  (params (GameEventOwnerCharacter :type Pawn%20Object%20Reference) (GameEventOwner :type Controller%20Object%20Reference))
  (Collision|UnbindEventfromOnActorBeginOverlap GameEventOwnerCharacter (delegate Custom|WhenBeginOverlap))
  (EventDispatchers|UnbindEventfromOnActorEndOverlap GameEventOwnerCharacter (delegate Custom|WhenEndOverlap)))

(fn ReceiveGetDescribe
  (return (Utilities|Text|FormatText "Need Reach {0} {1}" (Utilities|Text|ToText(String) (Utilities|GetDisplayName (Utilities|ResolveSoftReference (Variables|Default|Get目标)))) (Utilities|Text|ToText(String) (Utilities|String|SelectString "Finished!" "Unfinished!" (Class|XDGameEventElementBase|IsFinished))))))