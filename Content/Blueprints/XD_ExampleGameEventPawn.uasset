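; Example pawn that displays the state of the XD game event system on two text render components, one for underway events and one for finished events.
; Every Tick it passes both lists from XDGameEventManager to 更新游戏事件信息 (update game event info).
; That function walks each event's current sequences and their elements, concatenates names and descriptions, and sets the titled result as the text.
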(event EventBeginPlay)

(event Collision|EventActorBeginOverlap
  (params (OtherActor :type Actor%20Object%20Reference)))

(event EventTick
  (params (DeltaSeconds :type Float%20%28single-precision%29))
  (bind _xd_gameeventmanager (Variables|Default|GetXD_GameEventManager))
  (CallFunction|更新游戏事件信息 (Variables|Default|GetTextRender_Underway) (Variables|/Script/XD_GameEventSystem.XD_GameEventManager|GetUnderwayGameEventList _xd_gameeventmanager) "Underway 
")
  (CallFunction|更新游戏事件信息 (Variables|Default|GetTextRender_Finish) (Variables|/Script/XD_GameEventSystem.XD_GameEventManager|GetFinishGameEventList _xd_gameeventmanager) "Finish 
"))

(fn ConstructionScript)

(fn 更新游戏事件信息
  (params (TextRender :type Text%20Render%20Component%20Object%20Reference) (EventList :type Array%20of%20XD%20Game%20Event%20Base%20Object%20References) (Title :type String))
  (for _array_element EventList
    (bind _output_get (LocalVariables|SetResult (Utilities|String|Append (stale _output_get) (Utilities|String|ToString(Text) (Class|XDGameEventBase|GetGameEventName _array_element)) " 
")))
    (for _array_element_2 (Variables|/Script/XD_GameEventSystem.XD_GameEventBase|GetCurrentGameEventSequenceList _array_element)
      (bind _output_get_2 (LocalVariables|SetResult (Utilities|String|Append (stale _output_get_2) (Utilities|String|ToString(Text) (Class|XDGameEventSequenceBase|GetDescribe _array_element_2)) " 
")))
      (for _array_element_3 (Variables|/Script/XD_GameEventSystem.XD_GameEventSequenceBase|GetGameEventElementList _array_element_2)
        (bind _output_get_3 (LocalVariables|SetResult (Utilities|String|Append (stale _output_get_3) (Utilities|String|ToString(Text) (Class|XDGameEventElementBase|GetDescribe _array_element_3)) " 
"))))))
  (Rendering|Components|TextRender|SetText TextRender (Utilities|Text|ToText(String) (Utilities|String|Append Title (LocalVariables|GetResult)))))